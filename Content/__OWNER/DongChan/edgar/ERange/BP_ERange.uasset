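; BP_ERange is a short-lived range area actor tied to Edgar's E, which flags whether a BP_Edgar is inside it.
; On BeginPlay it sets a four-second lifespan.
; Actor begin and end overlap events pass the other actor to custom events that cast to BP_Edgar and set its IsEOverlap flag true on entry and false on exit.
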(event Custom|EndOverlap
  (params (Object :type Object%20Object%20Reference))
  (bind _asbp_edgar (Utilities|Casting|CastToBP_Edgar Object))
  (Variables|/Game/__OWNER/DongChan/Blueprint/BP_Edgar.BP_Edgar_C|SetbIsEOverlap? _asbp_edgar false))

(event Custom|BeginOverlap
  (params (Object :type Object%20Object%20Reference))
  (bind _asbp_edgar (Utilities|Casting|CastToBP_Edgar Object))
  (Variables|/Game/__OWNER/DongChan/Blueprint/BP_Edgar.BP_Edgar_C|SetbIsEOverlap? _asbp_edgar true))

(event EventBeginPlay
  (Actor|SetLifeSpan 4.0))

(event Collision|EventActorBeginOverlap
  (params (OtherActor :type Actor%20Object%20Reference))
  (CallFunction|BeginOverlap OtherActor))

(event Collision|EventActorEndOverlap
  (params (OtherActor :type Actor%20Object%20Reference))
  (CallFunction|EndOverlap OtherActor))

(fn ConstructionScript)