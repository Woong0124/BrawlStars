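; BP_Max_QSkill_Child is a spawner actor for Max's Q skill, firing three copies of BP_Max_QSkill at once.
; On BeginPlay it spawns one skill actor at each of three ChildActor components' world transforms, passing along its own owner and always spawning despite collisions.
; It then plays the Q skill sound with spatial attenuation at the first ChildActor's location, starting slightly into the clip.
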(event EventBeginPlay
  (bind _childactor (Variables|Default|GetChildActor))
  (bind _childactor1 (Variables|Default|GetChildActor1))
  (bind _childactor2 (Variables|Default|GetChildActor2))
  (bind _returnvalue (Transformation|GetWorldTransform _childactor1))
  (bind _returnvalue_2 (Transformation|GetWorldTransform _childactor))
  (bind _returnvalue_3 (Transformation|GetWorldTransform _childactor2))
  (Game|SpawnActorfromClass "/Game/__OWNER/SYL/BluePrints/BP_Max_QSkill.BP_Max_QSkill_C" (Math|Transform|MakeTransform (.location _returnvalue_2) (.rotation _returnvalue_2) (.scale _returnvalue_2)) "AdjustIfPossibleButAlwaysSpawn" (Components|GetOwner) 0)
  (Game|SpawnActorfromClass "/Game/__OWNER/SYL/BluePrints/BP_Max_QSkill.BP_Max_QSkill_C" (Math|Transform|MakeTransform (.location _returnvalue_3) (.rotation _returnvalue_3) (.scale _returnvalue_3)) "AdjustIfPossibleButAlwaysSpawn" (Components|GetOwner) 0)
  (Game|SpawnActorfromClass "/Game/__OWNER/SYL/BluePrints/BP_Max_QSkill.BP_Max_QSkill_C" (Math|Transform|MakeTransform (.location _returnvalue) (.rotation _returnvalue) (.scale _returnvalue)) "AdjustIfPossibleButAlwaysSpawn" (Components|GetOwner) 0)
  (Audio|SpawnSoundatLocation "/Game/__OWNER/Woong/Sound/Character/Max/Sound_MaxSkillQ.Sound_MaxSkillQ" (Transformation|GetSocketLocation (Variables|Default|GetChildActor) "None") "0, 0, 0" 1.0 1.0 0.19 "/Game/__OWNER/Woong/Sound/SA_SoundLocation.SA_SoundLocation" 0))

(fn ConstructionScript)