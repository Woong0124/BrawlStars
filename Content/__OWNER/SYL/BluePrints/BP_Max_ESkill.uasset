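; BP_Max_ESkill is the actor for Max's E skill, which explodes when its Sphere component hits something.
; BeginPlay calls a spawn-sound node with no sound asset shown.
; The first hit, gated by DoOnce, spawns a Niagara effect and attenuated sound at the actor's location.
; It then spawns BP_Max_ESkill_ExplosionRange at its transform, passing along its owner, and destroys itself.
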(event OnComponentHit(Sphere)
  (params (HitComponent :type Primitive%20Component%20Object%20Reference) (OtherActor :type Actor%20Object%20Reference) (OtherComp :type Primitive%20Component%20Object%20Reference) (NormalImpulse :type Vector :default "0, 0, 0") (Hit :type Hit%20Result%20Structure%20%28by%20ref%29))
  (Utilities|FlowControl|DoOnce false
    (:Completed
      (Niagara|SpawnSystematLocation "/Game/__OWNER/SYL/FX/NS_Max_ESkill.NS_Max_ESkill" (Transformation|GetActorLocation))
      (Audio|SpawnSoundatLocation "/Game/__OWNER/Woong/Sound/Character/Max/Sound_MaxSkillE.Sound_MaxSkillE" (Transformation|GetActorLocation) "0, 0, 0" 1.0 1.0 0.13 "/Game/__OWNER/Woong/Sound/SA_SoundLocation.SA_SoundLocation" 0)
      (Game|SpawnActorfromClass "/Game/__OWNER/SYL/BluePrints/BP_Max_ESkill_ExplosionRange.BP_Max_ESkill_ExplosionRange_C" (Transformation|GetActorTransform) "Undefined" (Components|GetOwner) 0)
      (Actor|DestroyActor))))

(event EventBeginPlay
  (Audio|SpawnSoundatLocation 0 "0, 0, 0" "0, 0, 0" 1.0 1.0 0.0 0 0))

(fn ConstructionScript)