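; W-skill projectile that damages a character it strikes.
; Tick spins Sphere1, while BeginPlay waits briefly, launches the actor along local negative X through ProjectileMovement, then destroys it after a short flight.
; Hits on anything except player zero spawn the NS_WSkill effect and destroy it.
; Capsule overlaps with non-owner characters spawn that effect, then a cast chain over four character Blueprints subtracts Damage from HP and destroys the projectile.
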(event OnComponentHit(Sphere)
  (params (HitComponent :type Primitive%20Component%20Object%20Reference) (OtherActor :type Actor%20Object%20Reference) (OtherComp :type Primitive%20Component%20Object%20Reference) (NormalImpulse :type Vector :default "0, 0, 0") (Hit :type Hit%20Result%20Structure%20%28by%20ref%29))
  (if (not (== OtherActor (Game|GetPlayerCharacter 0)))
    (Niagara|SpawnSystematLocation "/Game/__OWNER/SYL/FX/NS_WSkill.NS_WSkill" (Transformation|GetActorLocation))
    (Actor|DestroyActor)))

(event OnComponentBeginOverlap(Sphere)
  (params (OverlappedComponent :type Primitive%20Component%20Object%20Reference) (OtherActor :type Actor%20Object%20Reference) (OtherComp :type Primitive%20Component%20Object%20Reference) (OtherBodyIndex :type Integer) (bFromSweep :type Boolean) (SweepResult :type Hit%20Result%20Structure%20%28by%20ref%29))
  (bind _ascharacter (Utilities|Casting|CastToCharacter OtherActor))
  (if (Class|PrimitiveComponent|IsOverlappingComponent (Variables|/Script/Engine.Character|GetCapsuleComponent _ascharacter) (Variables|Default|GetSphere))
    (if (not (== OtherActor (Components|GetOwner)))
      (Variables|Default|SetEnemy%20Actor _ascharacter)
      (Niagara|SpawnSystematLocation "/Game/__OWNER/SYL/FX/NS_WSkill.NS_WSkill" (Transformation|GetActorLocation))
      (bind _asbp_max (Utilities|Casting|CastToBP_Max (Variables|Default|GetEnemy%20Actor))
        (:then
          (Variables|/Game/__OWNER/SYL/Character/BP_Max.BP_Max_C|SetCurrentHP _asbp_max (- (Variables|/Game/__OWNER/SYL/Character/BP_Max.BP_Max_C|GetCurrentHP _asbp_max) (Variables|Default|GetDamage)))
          (Actor|DestroyActor))
        (:CastFailed
          (bind _asamber_bp (Utilities|Casting|CastToAmber_BP (Variables|Default|GetEnemy%20Actor))
            (:then
              (bind _output_get (Variables|/Game/__OWNER/Rudals/Blueprints/Amber_BP.Amber_BP_C|SetCurrentHP _asamber_bp (- (Variables|/Game/__OWNER/Rudals/Blueprints/Amber_BP.Amber_BP_C|GetCurrentHP _asamber_bp) (Variables|Default|GetDamage))))
              (Development|PrintString (Utilities|String|ToString(Float) _output_get))
              (Actor|DestroyActor))
            (:CastFailed
              (bind _asbp_edgar (Utilities|Casting|CastToBP_Edgar (Variables|Default|GetEnemy%20Actor))
                (:then
                  (Variables|/Game/__OWNER/DongChan/Blueprint/BP_Edgar.BP_Edgar_C|SetCurrentHP _asbp_edgar (- (Variables|/Game/__OWNER/DongChan/Blueprint/BP_Edgar.BP_Edgar_C|GetCurrentHP _asbp_edgar) (Variables|Default|GetDamage)))
                  (Actor|DestroyActor))
                (:CastFailed
                  (bind _asbp_character_lou (Utilities|Casting|CastToBP_Character_LOU (Variables|Default|GetEnemy%20Actor)))
                  (Variables|/Game/__OWNER/Woong/Character/Blueprints/BP_Character_LOU.BP_Character_LOU_C|SetCurrentHp _asbp_character_lou (- (Variables|/Game/__OWNER/Woong/Character/Blueprints/BP_Character_LOU.BP_Character_LOU_C|GetCurrentHp _asbp_character_lou) (Variables|Default|GetDamage)))
                  (Actor|DestroyActor))))))))))

(event EventBeginPlay
  (Utilities|FlowControl|Delay 0.7)
  (Game|Components|ProjectileMovement|SetVelocityinLocalSpace (Variables|Default|GetProjectileMovement) "-1000.000000, 0, 0")
  (Utilities|FlowControl|Delay 0.65)
  (Actor|DestroyActor))

(event EventTick
  (params (DeltaSeconds :type Float%20%28single-precision%29))
  (Variables|Default|SetDelta%20Seconds (+ DeltaSeconds (Variables|Default|GetDelta%20Seconds)))
  (if (>= (Variables|Default|GetDelta%20Seconds) 0.02)
    (Transformation|AddRelativeRotation (Variables|Default|GetSphere1) "0,50.000000,0.000000" false false)
    (Variables|Default|SetDelta%20Seconds 0.0)))

(fn ConstructionScript)