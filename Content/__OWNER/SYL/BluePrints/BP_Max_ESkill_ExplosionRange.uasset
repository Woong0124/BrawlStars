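; Short-lived explosion damage volume for Max's E skill, which destroys itself a fraction of a second after spawning.
; Its sphere overlap checks for a Character's capsule, and a DoOnce limits the damage to the first such character.
; A cast chain over Max, Amber, Edgar and LOU sets LastDamageActor to the owner, subtracts Damage from HP directly and prints the result.
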(event OnComponentBeginOverlap(Sphere)
  (params (OverlappedComponent :type Primitive%20Component%20Object%20Reference) (OtherActor :type Actor%20Object%20Reference) (OtherComp :type Primitive%20Component%20Object%20Reference) (OtherBodyIndex :type Integer) (bFromSweep :type Boolean) (SweepResult :type Hit%20Result%20Structure%20%28by%20ref%29))
  (bind _ascharacter (Utilities|Casting|CastToCharacter OtherActor))
  (if (Class|PrimitiveComponent|IsOverlappingComponent (Variables|/Script/Engine.Character|GetCapsuleComponent _ascharacter) (Variables|Default|GetSphere))
    (Variables|Default|SetEnemy%20Actor _ascharacter)
    (Utilities|FlowControl|DoOnce false
      (:Completed
        (bind _asbp_character_max (Utilities|Casting|CastToBP_Character_Max (Variables|Default|GetEnemy%20Actor))
          (:then
            (Variables|/Game/__OWNER/SYL/Character/BP_Character_Max.BP_Character_Max_C|SetLastDamageActor _asbp_character_max (Components|GetOwner))
            (bind _output_get (Variables|/Game/__OWNER/SYL/Character/BP_Character_Max.BP_Character_Max_C|SetCurrentHP _asbp_character_max (- (Variables|/Game/__OWNER/SYL/Character/BP_Character_Max.BP_Character_Max_C|GetCurrentHP _asbp_character_max) (Variables|Default|GetDamage))))
            (Development|PrintString (Utilities|String|ToString(Float) _output_get)))
          (:CastFailed
            (bind _asamber_bp (Utilities|Casting|CastToAmber_BP (Variables|Default|GetEnemy%20Actor))
              (:then
                (Variables|/Game/__OWNER/Rudals/Blueprints/Amber_BP.Amber_BP_C|SetLastDamageActor _asamber_bp (Components|GetOwner))
                (bind _output_get_2 (Variables|/Game/__OWNER/Rudals/Blueprints/Amber_BP.Amber_BP_C|SetCurrentHP _asamber_bp (- (Variables|/Game/__OWNER/Rudals/Blueprints/Amber_BP.Amber_BP_C|GetCurrentHP _asamber_bp) (Variables|Default|GetDamage))))
                (Development|PrintString (Utilities|String|ToString(Float) _output_get_2)))
              (:CastFailed
                (bind _asbp_edgar (Utilities|Casting|CastToBP_Edgar (Variables|Default|GetEnemy%20Actor))
                  (:then
                    (Variables|/Game/__OWNER/DongChan/Blueprint/BP_Edgar.BP_Edgar_C|SetLastDamageActor _asbp_edgar (Components|GetOwner))
                    (bind _output_get_3 (Variables|/Game/__OWNER/DongChan/Blueprint/BP_Edgar.BP_Edgar_C|SetCurrentHP _asbp_edgar (- (Variables|/Game/__OWNER/DongChan/Blueprint/BP_Edgar.BP_Edgar_C|GetCurrentHP _asbp_edgar) (Variables|Default|GetDamage))))
                    (Development|PrintString (Utilities|String|ToString(Float) _output_get_3)))
                  (:CastFailed
                    (bind _asbp_character_lou (Utilities|Casting|CastToBP_Character_LOU (Variables|Default|GetEnemy%20Actor)))
                    (Variables|/Game/__OWNER/Woong/Character/Blueprints/BP_Character_LOU.BP_Character_LOU_C|SetLastDamageActor _asbp_character_lou (Components|GetOwner))
                    (bind _output_get_4 (Variables|/Game/__OWNER/Woong/Character/Blueprints/BP_Character_LOU.BP_Character_LOU_C|SetCurrentHp _asbp_character_lou (- (Variables|/Game/__OWNER/Woong/Character/Blueprints/BP_Character_LOU.BP_Character_LOU_C|GetCurrentHp _asbp_character_lou) (Variables|Default|GetDamage))))
                    (Development|PrintString (Utilities|String|ToString(Float) _output_get_4))))))))))))

(event EventBeginPlay
  (Utilities|FlowControl|Delay 0.35)
  (Actor|DestroyActor))

(fn ConstructionScript)