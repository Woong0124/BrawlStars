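; Grass map-dressing Blueprint, by its name a descendant of BP_Grass, that lays out a small fixed grid of mesh instances.
; The Construction Script runs two loops that add Hierarchical Instanced Static Mesh instances in two parallel rows along Y, spaced about 110 units apart.
; The event graph holds only disabled parent-call stubs, so this asset adds no runtime logic.
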(event EventBeginPlay
  (|CallParentFunction) ; 지금 이 노드는 비활성 상태입니다. \n핀을 끌어서 다른 노드를 연결하면 활성화됩니다.
)

(event Collision|EventActorBeginOverlap
  (params (OtherActor :type Actor%20Object%20Reference))
  (|CallParentFunction OtherActor) ; 지금 이 노드는 비활성 상태입니다. \n핀을 끌어서 다른 노드를 연결하면 활성화됩니다.
)

(event EventTick
  (params (DeltaSeconds :type Float%20%28single-precision%29))
  (|CallParentFunction DeltaSeconds) ; 지금 이 노드는 비활성 상태입니다. \n핀을 끌어서 다른 노드를 연결하면 활성화됩니다.
)

(fn ConstructionScript
  (for _index (range 0 2)
    (Components|InstancedStaticMesh|AddInstance (Variables|Default|GetHierarchicalInstancedStaticMesh) (Math|Transform|MakeTransform (Math|Vector|MakeVector 0.0 (* _index 111.0) 0.0))))
  (for _index_2 (range 0 2)
    (Components|InstancedStaticMesh|AddInstance (Variables|Default|GetHierarchicalInstancedStaticMesh) (Math|Transform|MakeTransform (Math|Vector|MakeVector 1.1e+02 (* _index_2 111.0) 0.0)))))