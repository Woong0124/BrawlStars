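; BP_Skill is a short-lived skill hit actor that damages Amber_BP characters overlapping its Sphere, then destroys itself 0.2 seconds after spawning.
; The construction script caches the owner so the overlap check can exclude it, and only hits on the character's capsule count.
; A hit subtracts the victim's own QDamage from its CurrentHP and sets the first PlayerStateManager status flag, preserving the toxicating and slowing flags.
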(event OnComponentBeginOverlap(Sphere)
  (params (OverlappedComponent :type Primitive%20Component%20Object%20Reference) (OtherActor :type Actor%20Object%20Reference) (OtherComp :type Primitive%20Component%20Object%20Reference) (OtherBodyIndex :type Integer) (bFromSweep :type Boolean) (SweepResult :type Hit%20Result%20Structure%20%28by%20ref%29))
  (bind _output_get (Variables|Default|SetEnemyActor OtherActor))
  (bind _ascharacter (Utilities|Casting|CastToCharacter _output_get))
  (if (Class|PrimitiveComponent|IsOverlappingComponent (Variables|/Script/Engine.Character|GetCapsuleComponent _ascharacter) (Variables|Default|GetSphere))
    (if (not (== (Variables|Default|GetEnemyActor) (Variables|Default|GetOwnerActor)))
      (bind _asamber_bp (Utilities|Casting|CastToAmber_BP (Variables|Default|GetEnemyActor)))
      (Variables|/Game/__OWNER/Rudals/Blueprints/Amber_BP.Amber_BP_C|SetCurrentHP _asamber_bp (- (Variables|/Game/__OWNER/Rudals/Blueprints/Amber_BP.Amber_BP_C|GetCurrentHP _asamber_bp) (Variables|/Game/__OWNER/Rudals/Blueprints/Amber_BP.Amber_BP_C|GetQ_Damage _asamber_bp)))
      (Variables|/Game/__OWNER/Rudals/Blueprints/Amber_BP.Amber_BP_C|SetPlayerStateManager _asamber_bp (Utilities|Struct|MakeS_PlayerState true (.bistoxicating (Variables|/Game/__OWNER/Rudals/Blueprints/Amber_BP.Amber_BP_C|GetPlayerStateManager _asamber_bp)) (.bisslowing (Variables|/Game/__OWNER/Rudals/Blueprints/Amber_BP.Amber_BP_C|GetPlayerStateManager _asamber_bp)))))))

(event EventBeginPlay
  (Utilities|FlowControl|Delay 0.2)
  (Actor|DestroyActor))

(event Collision|EventActorBeginOverlap
  (params (OtherActor :type Actor%20Object%20Reference)))

(event EventTick
  (params (DeltaSeconds :type Float%20%28single-precision%29)))

(fn ConstructionScript
  (Variables|Default|SetOwnerActor (Components|GetOwner self)))