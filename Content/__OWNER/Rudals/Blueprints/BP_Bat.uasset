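; BP_Bat is a lifesteal skill bat that destroys itself after ten seconds.
; On capsule overlap with an Amber_BP other than its cached instigator, it subtracts the victim's own EDamage from that victim's CurrentHP.
; It then heals the instigator by the instigator's EDamage, capped at MaxHP, and destroys itself.
; UpdateWalkSpeed sets its movement speed, and the NS_E_Skill Niagara spawn is left unconnected.
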(event OnComponentBeginOverlap(CapsuleComponent)
  (params (OverlappedComponent :type Primitive%20Component%20Object%20Reference) (OtherActor :type Actor%20Object%20Reference) (OtherComp :type Primitive%20Component%20Object%20Reference) (OtherBodyIndex :type Integer) (bFromSweep :type Boolean) (SweepResult :type Hit%20Result%20Structure%20%28by%20ref%29))
  (bind _output_get (Variables|Default|SetEnemyActor OtherActor))
  (bind _ascharacter (Utilities|Casting|CastToCharacter _output_get))
  (if (Class|PrimitiveComponent|IsOverlappingComponent (Variables|/Script/Engine.Character|GetCapsuleComponent _ascharacter) (Variables|Collision|GetCapsuleComponent))
    (if (not (== (Variables|Default|GetEnemyActor) (Variables|Default|GetInstigatorActor)))
      (bind _asamber_bp (Utilities|Casting|CastToAmber_BP (Variables|Default|GetEnemyActor)))
      (Variables|/Game/__OWNER/Rudals/Blueprints/Amber_BP.Amber_BP_C|SetCurrentHP _asamber_bp (- (Variables|/Game/__OWNER/Rudals/Blueprints/Amber_BP.Amber_BP_C|GetCurrentHP _asamber_bp) (Variables|/Game/__OWNER/Rudals/Blueprints/Amber_BP.Amber_BP_C|GetE_Damage _asamber_bp)))
      (bind _asamber_bp_2 (Utilities|Casting|CastToAmber_BP (Variables|Default|GetInstigatorActor)))
      (if (> (Variables|/Game/__OWNER/Rudals/Blueprints/Amber_BP.Amber_BP_C|GetMaxHP _asamber_bp_2) (+ (Variables|/Game/__OWNER/Rudals/Blueprints/Amber_BP.Amber_BP_C|GetCurrentHP _asamber_bp_2) (Variables|/Game/__OWNER/Rudals/Blueprints/Amber_BP.Amber_BP_C|GetE_Damage _asamber_bp_2)))
        (Variables|/Game/__OWNER/Rudals/Blueprints/Amber_BP.Amber_BP_C|SetCurrentHP _asamber_bp_2 (+ (Variables|/Game/__OWNER/Rudals/Blueprints/Amber_BP.Amber_BP_C|GetCurrentHP _asamber_bp_2) (Variables|/Game/__OWNER/Rudals/Blueprints/Amber_BP.Amber_BP_C|GetE_Damage _asamber_bp_2)))
        (Actor|DestroyActor)
        (else
          (Variables|/Game/__OWNER/Rudals/Blueprints/Amber_BP.Amber_BP_C|SetCurrentHP _asamber_bp_2 (Variables|/Game/__OWNER/Rudals/Blueprints/Amber_BP.Amber_BP_C|GetMaxHP _asamber_bp_2))
          (Actor|DestroyActor))))))

(event EventBeginPlay
  (Utilities|FlowControl|Delay 1e+01)
  (Actor|DestroyActor))

(event EventTick
  (params (DeltaSeconds :type Float%20%28single-precision%29)))

(fn ConstructionScript
  (Variables|Default|SetInstigatorActor (Game|GetInstigator self)))

(fn UpdateWalkSpeed
  (params (NewWalkSpeed :type Float%20%28single-precision%29))
  (Variables|/Script/Engine.CharacterMovementComponent|SetMaxWalkSpeed (Variables|Character|GetCharacterMovement) NewWalkSpeed))