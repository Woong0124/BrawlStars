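; Player character Lou, with cursor-aimed Q/W/E skills, an HP widget and a timed slow debuff.
; Q uses recharging charges to fire twice, turning toward the cursor; W launches a projectile that bursts into Niagara blizzard effects and a collision actor at the saved cursor point or on death.
; Holding E briefly raises speed, shows an effect and prints HP-recovery messages, while Gates block Q and W.
; Tick updates the cursor, W arrival, Q recharge and slow.
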(event Custom|E_SkillW
  ;[1 1 1] W Skill Do
  ;[0.4161 0.3633 0.7469] 1
  (CallFunction|ESkillWFindMouse))

(event Custom|E_SkillQ
  ;[1 1 1] Q Skill Do
  ;[1 0.4435 0.9757] 1
  (CallFunction|ESkillQFindRotate)
  (Utilities|FlowControl|Delay 0.2)
  ;[0.6427 0 0.6147] 3
  (CallFunction|ESkillQReplay))

(event Custom|E_SkillQ_Replay
  ;[0.6427 0 0.6147] 3
  ;[0.8094 0.1172 0.7792] 2, 4
  (CallFunction|ESkillQTurnandSpawnSkill (stale Custom|E_SkillQ_FindRotate _rotation)))

(event Custom|E_SkillW_FindMouse
  ;[0.4161 0.3633 0.7469] 1
  (bind _location (CallFunction|SaveCursortoWorld))
  (Variables|Default|SetSaveParticleSpawnPoint _location)
  (bind _rotation (CallFunction|FindActortoMouseRotation))
  ;[0.103 0.07998 0.2469] 2
  (CallFunction|ESkillWTurnandSpawnSkill _rotation))

(event Custom|E_SkillW_TurnAndSpawnSkill
  (params (NewRelativeRotation :type Rotator))
  ;[0.103 0.07998 0.2469] 2
  (CallFunction|TurnActor NewRelativeRotation)
  (bind _spawnskillreturnvalue (Spawn|SpawnSkillTargetVer (Variables|Default|GetC_RefSkillW) (Variables|Default|GetSkillArrowPoint)))
  (Variables|Default|SetSkillW _spawnskillreturnvalue))

(event Custom|E_SkillE_GateOn
  (params (Condition :type Boolean))
  (Variables|/Script/Engine.CharacterMovementComponent|SetMaxWalkSpeed (Variables|Character|GetCharacterMovement) 3.8e+02)
  (디폴트|SkillVisibility Condition)
  (Development|PrintString "HP회복 시작" true true "(R=0.182503,G=0.591667,B=0.400506,A=1.000000)")
  (Utilities|FlowControl|Sequence
    (:then_0
      (Utilities|FlowControl|Gate false) ; enters at Close
    )
    (:then_1
      (Utilities|FlowControl|Gate false) ; enters at Close
    )))

(event Custom|E_SkillE_GateOff
  (params (Condition :type Boolean))
  (Variables|/Script/Engine.CharacterMovementComponent|SetMaxWalkSpeed (Variables|Character|GetCharacterMovement) 3e+02)
  (디폴트|SkillVisibility Condition)
  (Development|PrintString "HP회복 끝" true true "(R=1.000000,G=0.387500,B=0.387500,A=1.000000)")
  (Utilities|FlowControl|Sequence
    (:then_0
      (Utilities|FlowControl|Gate false) ; enters at Open
    )
    (:then_1
      (Utilities|FlowControl|Gate false) ; enters at Open
    )))

(event Custom|E_SkillE_Off
  ;[1 1 1] E Skill Off
  (bind _output_get (Variables|Default|SetbSkillE_Visibility false))
  (CallFunction|ESkillEGateOff _output_get))

(event Custom|E_CoolTimeW
  ;[0 0 0] 쿨타임
  (Variables|Default|SetbCoolTime_W true)
  (Utilities|FlowControl|Delay 9.0)
  (Variables|Default|SetbCoolTime_W false))

(event Custom|E_CoolTimeE
  ;[0 0 0] 쿨타임
  (Utilities|FlowControl|Delay 7.0)
  (Variables|Default|SetbCoolTime_E false))

(event Custom|E_SkillQ_Cheak
  (Utilities|FlowControl|Gate false
    (:Exit
      (if (>= (Variables|Default|GetCoolTime_Q) 1)
        (CallFunction|ESkillQ)
        ;[0 0 0] 쿨타임
        (Variables|Default|SetCoolTime_Q (- (Variables|Default|GetCoolTime_Q) 1))))))

(event Custom|E_SkillW_Particle
  (params (SpawnLocation :type Vector))
  ;[1 1 1] Lou Skill W 나이아가라 파티클 생성
  (스폰|SpawnSkillParticle SpawnLocation "/Game/__OWNER/Woong/FX/NP_LouSkillW_Blizzard.NP_LouSkillW_Blizzard" "/Game/__OWNER/Woong/FX/NP_LouSkillW_Ground.NP_LouSkillW_Ground" "/Game/__OWNER/Woong/FX/NP_LouSkillW_Smoke.NP_LouSkillW_Smoke"))

(event Custom|E_SkillW_Cheak
  (Utilities|FlowControl|Gate false
    (:Exit
      (if (not (Variables|Default|GetbCoolTime_W))
        (CallFunction|ESkillW)
        ;[0 0 0] 쿨타임
        (CallFunction|ECoolTimeW)))))

(event Custom|E_SkillW_Collision
  (params (Location :type Vector))
  ;[1 1 1] Lou Skill W Collision 생성
  (스폰|SpawnSkillLocationVer (Variables|Default|GetC_RefSkillW_Collision) Location))

(event Custom|E_SkillQ_FindRotate
  ;[1 0.4435 0.9757] 1
  (bind _rotation (CallFunction|FindActortoMouseRotation))
  ;[0.8094 0.1172 0.7792] 2, 4
  (CallFunction|ESkillQTurnandSpawnSkill _rotation))

(event Custom|E_SkillW_Spawn
  ;[1 0.933 0.4666] 수명이 다하거나, 벽에 Hit 되었을 때
  (bind _output_get (Variables|Default|SetSaveParticleSpawnPoint (Transformation|GetActorLocation (Variables|Default|GetSkillW))))
  (CallFunction|ESkillWParticle _output_get)
  (CallFunction|ESkillWCollision _output_get)
  (Actor|DestroyActor (Variables|Default|GetSkillW)))

(event Custom|E_SkillW_Dead
  ;[1 1 1] 수명이 다하거나, 벽에 Hit 되었을 때, (BP_SkillW)
  (CallFunction|ESkillWSpawn))

(event Custom|E_SkillQ_TurnAndSpawnSkill
  (params (NewRelativeRotation :type Rotator))
  ;[0.8094 0.1172 0.7792] 2, 4
  (CallFunction|TurnActor NewRelativeRotation)
  (Spawn|SpawnSkillTargetVer (Variables|Default|GetC_RefSkillQ) (Variables|Default|GetSkillArrowPoint)))

(event Custom|E_SkillE_On
  ;[1 1 1] E Skill On
  (bind _output_get (Variables|Default|SetbSkillE_Visibility true))
  (CallFunction|ESkillEGateon _output_get))

(event EventBeginPlay
  (Variables|Default|SetCurrentHp (Variables|Default|GetMaxHp))
  (bind _asumg_player_interface (Utilities|Casting|CastToUMG_PlayerInterface (UserInterface|GetUserWidgetObject (Variables|Default|GetHpUi))))
  (bind _output_get (Variables|Default|SetUMG_Player_Interface _asumg_player_interface))
  (Variables|/Game/__OWNER/Rudals/UI/UMG_PlayerInterface.UMG_PlayerInterface_C|SetOwnerActor _output_get self)
  (Variables|Default|SetPlayerStateManager (Utilities|Struct|MakeS_PlayerState false false false)))

(event EventTick
  (params (DeltaSeconds :type Float%20%28single-precision%29))
  (bind _skillw (Variables|Default|GetSkillW))
  ;[1 1 1] Tick
  (Utilities|FlowControl|Sequence
    (:then_0
      ;[1 1 1] 커서의 위치를 저장
      (CallFunction|SaveCursortoWorld)
      (Components|SkinnedMesh|HideBonebyName (Variables|Character|GetMesh) "L_gunbone_01_s" "PBO_Term"))
    (:then_1
      ;[1 1 1] W 활성화 시, 실행
      (Utilities|IsValid _skillw
        (:Is%20Valid
          (if (Math|Vector|Equal(Vector) (Transformation|GetActorLocation _skillw) (Variables|Default|GetSaveParticleSpawnPoint) 8e+01)
            (CallFunction|ESkillWSpawn)))))
    (:then_2
      ;[0 0 0] 쿨타임
      (if (not (>= (Variables|Default|GetCoolTime_Q) 3))
        (Utilities|FlowControl|Delay 2.2)
        (Variables|Default|SetCoolTime_Q (+ (Variables|Default|GetCoolTime_Q) 1))))
    (:then_3
      (if (.bisslowing (Variables|Default|GetPlayerStateManager))
        (Variables|/Script/Engine.CharacterMovementComponent|SetMaxWalkSpeed (Variables|Character|GetCharacterMovement) 2.2e+02)
        (Variables|Default|SetPlayerStateManager (Utilities|Struct|MakeS_PlayerState (.bisblooding (Variables|Default|GetPlayerStateManager)) (.bistoxicating (Variables|Default|GetPlayerStateManager)) false))
        (Utilities|FlowControl|Delay 2.0)
        (Variables|/Script/Engine.CharacterMovementComponent|SetMaxWalkSpeed (Variables|Character|GetCharacterMovement) 3e+02)))))

(event Input|KeyboardEvents|Q
  (params (Key :type Key%20Structure :default "None"))
  ;[1 0 0.6399] Q Skill
  (:Pressed
    (CallFunction|ESkillQCheak)))

(event Input|KeyboardEvents|W
  (params (Key :type Key%20Structure :default "None"))
  ;[0.3166 0 1] W Skill
  (:Pressed
    (CallFunction|ESkillWCheak)))

(event Input|KeyboardEvents|E
  (params (Key :type Key%20Structure :default "None"))
  ;[0.01603 0.7235 1] E Skill
  (:Pressed
    (if (not (Variables|Default|GetbCoolTime_E))
      (Variables|Default|SetbCoolTime_E true)
      (CallFunction|ESkillEon)
      (Utilities|FlowControl|Delay 2.0)
      (CallFunction|ESkillEOff :!label _label)
      ;[0 0 0] 쿨타임
      (CallFunction|ECoolTimeE)))
  (:Released
    (goto _label)))

(fn ConstructionScript)

(fn TurnActor
  (params (NewRelativeRotation :type Rotator))
  ;[1 1 1 0] 액터를 마우스 포인터의 방향으로 턴
  (Transformation|SetActorRelativeRotation NewRelativeRotation))

(fn FindActortoMouseRotation
  (bind _self self)
  (bind _cursortoworld (Variables|Default|GetCursorToWorld))
  (bind _returnvalue (Transformation|GetWorldLocation _cursortoworld))
  (bind _returnvalue_2 (Transformation|GetActorLocation _self))
  ;[1 1 1 0] 액터와 마우스 사이의 회전값 저장
  (bind _output_get (Variables|Default|SetFindRotation (Math|Rotator|FindLookatRotation (Math|Vector|MakeVector (.x _returnvalue_2) (.y _returnvalue_2) (.z _returnvalue_2)) (Math|Vector|MakeVector (.x _returnvalue) (.y _returnvalue) (.z _returnvalue_2)))))
  (return _output_get))

(fn SpawnSkillTargetVer
  (params (SpawnSkillClass :type Actor%20Class%20Reference) (GetWorldLocationTarget :type Scene%20Component%20Object%20Reference))
  (bind _returnvalue (Transformation|GetActorTransform))
  (bind _self self)
  ;[1 1 1 0] 액터 스폰
  (bind _returnvalue_2 (Game|SpawnActorfromClass SpawnSkillClass (Math|Transform|MakeTransform (Transformation|GetWorldLocation GetWorldLocationTarget) (.rotation _returnvalue) (.scale _returnvalue)) "Undefined" _self _self))
  (return _returnvalue_2))

(fn SpawnSkillParticle
  (params (SpawnLocation :type Vector) (Particle1 :type Niagara%20System%20Object%20Reference) (Particle2 :type Niagara%20System%20Object%20Reference) (Particle3 :type Niagara%20System%20Object%20Reference))
  (bind _returnvalue (Niagara|SpawnSystematLocation Particle1 SpawnLocation))
  (bind _returnvalue_2 (Niagara|SpawnSystematLocation Particle2 SpawnLocation))
  (bind _returnvalue_3 (Niagara|SpawnSystematLocation Particle3 SpawnLocation))
  (return _returnvalue _returnvalue_2 _returnvalue_3))

(fn SpawnSkillLocationVer
  (params (SpawnSkillClass :type Actor%20Class%20Reference) (Location :type Vector))
  (bind _returnvalue (Transformation|GetActorTransform))
  (bind _self self)
  ;[1 1 1 0] 액터 스폰
  (bind _returnvalue_2 (Game|SpawnActorfromClass SpawnSkillClass (Math|Transform|MakeTransform Location (.rotation _returnvalue) (.scale _returnvalue)) "Undefined" _self _self))
  (return _returnvalue_2))

(fn SkillVisibility
  (params (Condition :type Boolean))
  (if Condition
    (Rendering|SetVisibility (Variables|Default|GetNP_LouSkillE) true false)
    (else
      (Rendering|SetVisibility (Variables|Default|GetNP_LouSkillE) false false))))

(fn SaveCursortoWorld
  (bind _returnvalue (Game|GetPlayerController 0))
  (bind _hitresult (Game|Player|GetHitResultUnderCursorbyChannel _returnvalue "TraceTypeQuery1" true))
  (bind (_bblockinghit _binitialoverlap _time _distance _location _impactpoint _normal _impactnormal) (Collision|BreakHitResult _hitresult))
  (Transformation|SetWorldLocationAndRotation (Variables|Default|GetCursorToWorld) _location (Math|Rotator|MakeRotationfromAxes _impactnormal "0, 0, 0" "0, 0, 0") false false)
  (return _location))

(fn AllinSpawnSkill
  (params (SpawnSkillClass :type Actor%20Class%20Reference) (GetWorldLocationTarget :type Scene%20Component%20Object%20Reference))
  ;[1 1 1] 마우스위치찾기+액터돌리기+스폰액터
  (bind _rotation (CallFunction|FindActortoMouseRotation))
  (CallFunction|TurnActor _rotation)
  (bind _spawnskillreturnvalue (Spawn|SpawnSkillTargetVer SpawnSkillClass GetWorldLocationTarget))
  (return _spawnskillreturnvalue))

(fn SetActivity
  (params (Condition :type Boolean))
  (if Condition
    (Components|Activation|SetActive (Variables|Character|GetCharacterMovement) false false)
    (else
      (Components|Activation|SetActive (Variables|Character|GetCharacterMovement) true true))))